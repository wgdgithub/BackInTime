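; Actor component that gives its owner a time-rewind ability, replaying recorded transform and physics motion in reverse.
; While not rewinding, Tick records location, rotation, static mesh velocities and delta time into a history buffer, trimmed at about ten seconds.
; UpdateBackTime toggles rewinding, which applies and removes the newest snapshot each tick until the buffer empties.
; Playback is frame-by-frame without interpolation, and adds each delta to the length counter rather than subtracting it.
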(event `self.ReceiveBeginPlay`
  (if (not (`self.InInited`))
    (set `self.InInited` true)
    (set `self.Owner` (`self.GetOwner`))))

(event `/Game/_Test/BPI_BackTime.UpdateBackTime`
  (params (IsBackTime :type Boolean))
  (set `self.IsBackTimeing` IsBackTime))

(event `self.ReceiveTick`
  (params (DeltaSeconds :type "Float (single-precision)"))
  (if (`self.InInited`)
    (if (`self.IsBackTimeing`)
      (if (not (`self.IsOutData`))
        (`self.ExcuTimeFrameInfo`))
      (else
        (`self.RecordTimeFrameInfo` DeltaSeconds)))))

(fn `ExcuTimeFrameInfo`
  (bind _timeframeinfo (`self.TimeFrameInfo`))
  (bind _timeframeinfo_2 (`self.TimeFrameInfo`))
  (bind (_output_location _output_rotation _output_linearvelocity _output_angularvelocity _output_deltatime) (break `/Game/_Test/S_TimeInfo` (`|GetArrayItem` _timeframeinfo (`KismetArrayLibrary.Array_LastIndex` _timeframeinfo))))
  (if (<= (`KismetArrayLibrary.Array_Length` (`self.TimeFrameInfo`)) 0)
    (set `self.BackTimeLength` 0.0)
    (set `self.IsOutData` true)
    (else
      (`Actor.K2_SetActorRotation` (`self.Owner`) _output_rotation false)
      (`Actor.K2_SetActorLocation` (`self.Owner`) _output_location false false)
      (`PrimitiveComponent.SetPhysicsLinearVelocity` (`Actor.GetComponentByClass` (`self.Owner`) "/Script/Engine.StaticMeshComponent") _output_linearvelocity false "None")
      (`PrimitiveComponent.SetAllPhysicsAngularVelocityInDegrees` (`Actor.GetComponentByClass` (`self.Owner`) "/Script/Engine.StaticMeshComponent") _output_angularvelocity false)
      (set `self.BackTimeLength` (+ (`self.BackTimeLength`) _output_deltatime))
      (`KismetArrayLibrary.Array_Remove` _timeframeinfo_2 (`KismetArrayLibrary.Array_LastIndex` _timeframeinfo_2)))))

(fn `RecordTimeFrameInfo`
  (params (`Delta Time` :type "Float (double-precision)"))
  (bind _owner (`self.Owner`))
  (bind _timeframeinfo (`self.TimeFrameInfo`))
  (bind _returnvalue (`Actor.GetComponentByClass` _owner "/Script/Engine.StaticMeshComponent"))
  (bind (_output_location _output_rotation _output_linearvelocity _output_angularvelocity _output_deltatime) (break `/Game/_Test/S_TimeInfo` (`|GetArrayItem` _timeframeinfo)))
  (`/Engine/EditorBlueprintResources/StandardMacros.IsValid` _returnvalue
    (:`Is Valid`
      (if (<= (`self.BackTimeLength`) 10.0)
        (bind _returnvalue_2 (`PrimitiveComponent.GetPhysicsLinearVelocity` _returnvalue "None"))
        (else
          (`KismetArrayLibrary.Array_Remove` _timeframeinfo)
          (set `self.BackTimeLength` (- (`self.BackTimeLength`) _output_deltatime))))
      (`KismetArrayLibrary.Array_Add` (`self.TimeFrameInfo`) (make `/Game/_Test/S_TimeInfo` (`Actor.K2_GetActorLocation` _owner) (`Actor.K2_GetActorRotation` _owner) _returnvalue_2 (`PrimitiveComponent.GetPhysicsAngularVelocityInDegrees` _returnvalue "None") `Delta Time`))
      (set `self.BackTimeLength` (+ `Delta Time` (`self.BackTimeLength`)))
      (set `self.IsOutData` false))))